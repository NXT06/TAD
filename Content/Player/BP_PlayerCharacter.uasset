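; Player pawn that floats and bobs on water, using FloatingPawnMovement with custom gravity, jumping, and move input that is ignored on land.
; Each Tick, a downward trace detects water (AC_Flow), walkable ground or air to set buoyancy or fall velocity.
; Tick also scales a traced blob shadow, writes player location to MPC_Global and sphere-traces for BPI_Interactable actors.
; Splash Niagara effects are registered with BP_RippleManager's scene capture for ripples.
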(event OnComponentBeginOverlap(Collision)
  (params (OverlappedComponent :type Primitive%20Component%20Object%20Reference) (OtherActor :type Actor%20Object%20Reference) (OtherComp :type Primitive%20Component%20Object%20Reference) (OtherBodyIndex :type Integer) (bFromSweep :type Boolean) (SweepResult :type Hit%20Result%20Structure%20%28by%20ref%29))
  (Development|PrintString "Hello"))

(event OnComponentBeginOverlap(Sphere)
  (params (OverlappedComponent :type Primitive%20Component%20Object%20Reference) (OtherActor :type Actor%20Object%20Reference) (OtherComp :type Primitive%20Component%20Object%20Reference) (OtherBodyIndex :type Integer) (bFromSweep :type Boolean) (SweepResult :type Hit%20Result%20Structure%20%28by%20ref%29))
  (Development|PrintString "Hello"))

(event Custom|CE_HandleGravity
  (bind _returnvalue (Transformation|GetActorLocation))
  ;[0.1202 0.0251 0.15 0.5] Gravity
  (Utilities|FlowControl|Sequence
    (:then_0
      (bind (_outhit _returnvalue_2) (Collision|LineTraceByChannel _returnvalue (- _returnvalue (Math|Vector|MakeVector 0.0 0.0 (+ (Components|Capsule|GetScaledCapsuleHalfHeight (Variables|Default|GetCollision)) 3e+01))) "TraceTypeQuery1" false 0 "None" true (Variables|Default|GetTrace%20Hit%20Color) (Variables|Default|GetTrace%20Hit%20Color)))
      (if _returnvalue_2
        (bind _result (CallFunction|CheckforWater _outhit))
        (if _result
          (Variables|Default|SetOnLand false)
          (Variables|Default|SetDistance (.Distance (Collision|BreakHitResult _outhit)))
          (if (< (.Distance (Collision|BreakHitResult _outhit)) (+ (Variables|/Script/Engine.CapsuleComponent|GetCapsuleHalfHeight (Variables|Default|GetCollision)) 1e+01))
            (Variables|Default|SetFloating true)
            (Variables|Default|SetGravityMult 0.0)
            (Variables|Default|SetJumpSpawn 5e+01)
            (CallFunction|AddVelocity 0.0 0.0 (* 1.0 (Variables|Default|GetFloatForce)))
            (Utilities|FlowControl|DoOnce false :!label _label
              (:Completed
                (bind _returnvalue_3 (Niagara|SpawnSystematLocation "/Game/VFX/NS_WaterSplash.NS_WaterSplash" (+ (Transformation|GetActorLocation) "0.000000,0.000000,20.000000") "0, 0, 0" "0.500000,0.500000,0.500000" false true "AutoRelease"))
                (Rendering|SceneCapture|ShowOnlyComponent (Variables|/Game/Landscapes/WorldInteraction/BP_RippleManager.BP_RippleManager_C|GetSceneCapture (Variables|Default|GetRippleManager)) _returnvalue_3)))
            (else
              (Variables|Default|SetFloating true)
              (Variables|Default|SetGravityMult 0.0)
              (Variables|Default|SetJumpSpawn 5e+01)
              (goto _label Reset)))
          (elif (< (Class|KismetMathLibrary|DegAcos (Math|Vector|DotProduct (.ImpactNormal (Collision|BreakHitResult _outhit)) (Math|Vector|GetUpVector (Variables|Default|GetCollision)))) 45.0)
            (Variables|Default|SetOnLand true)
            (CallFunction|CEStopBobing false)
            (Variables|Default|SetJumpSpawn 5.0)
            (bind _output_get (Variables|Default|SetGravityMult 0.1))
            (CallFunction|AddVelocity 0.0 0.0 (* _output_get (Variables|Default|GetFallSpeed) -1.0))
            (else
              (Variables|Default|SetFloating false :!label _label_2)
              (Variables|Default|SetOnLand false)
              (CallFunction|CEStopBobing true)
              (Variables|Default|SetGravityMult (+ (Variables|Default|GetGravityMult) (Variables|Default|GetDeltaTime)))
              (CallFunction|AddVelocity 0.0 0.0 (* (Variables|Default|GetGravityMult) (Variables|Default|GetFallSpeed) -1.0)))))
        (else
          (goto _label_2))))
    (:then_1
      ;;[0.15 0.15 0.15 0.5] Trace Color
      (if (Variables|Default|GetOnLand)
        (Variables|Default|SetTrace%20Hit%20Color "(R=0.004453,G=0.588167,B=1.000000,A=1.000000)")
        (elif (Variables|Default|GetFloating)
          (Variables|Default|SetTrace%20Hit%20Color "(R=0.025765,G=1.000000,B=0.184122,A=1.000000)")
          (else
            (Variables|Default|SetTrace%20Hit%20Color "(R=1.000000,G=0.000000,B=0.056839,A=1.000000)")))))))

(event Custom|CE_BobAnim
  ;[0.15 0.15 0.15 0.5] Bobing Animation
  (Input|AddMappingContext (PlayerController|LocalPlayerSubsystems|GetEnhancedInputLocalPlayerSubsystem (Game|GetPlayerController 0)) "/Game/Player/Input/I_PlayerControls.I_PlayerControls" 0 "(bIgnoreAllPressedKeysUntilRelease=True,bForceImmediately=False,bNotifyUserSettings=False)")
  (bind _bobing (Timeline|Bobing Play)
    (:Update
      (Transformation|SetRelativeLocation (Variables|Default|GetSphere) (Math|Vector|MakeVector 0.0 0.0 (* _bobing (Variables|Default|GetBobDist))) false false))))

(event Custom|CE_SetShadow
  (bind _returnvalue (Transformation|GetActorLocation))
  (bind _shadow (Variables|Default|GetShadow))
  ;[0.15 0.15 0.15 0.5] Update Shadow
  (bind _outhit (Collision|LineTraceByChannel (- _returnvalue "") (- _returnvalue "0.000000,0.000000,5000.000000") "TraceTypeQuery3" false 0 "None"))
  (Transformation|SetWorldLocation _shadow (.Location (Collision|BreakHitResult _outhit)) false true)
  (Transformation|SetRelativeScale3D _shadow (Math|Vector|MakeVector 1.0 (Math|Float|Clamp(Float) (- 1.0 (/ (- (.Distance (Collision|BreakHitResult _outhit)) 1.5e+02) 2e+02)) 0.25) (Math|Float|Clamp(Float) (- 1.0 (/ (- (.Distance (Collision|BreakHitResult _outhit)) 1.5e+02) 2e+02)) 0.25))))

(event Custom|CE_StopBobing
  (params (Start :type Boolean))
  (bind _bobing (Variables|Default|GetBobing))
  ;[0.15 0.15 0.15 0.5] Change Bobing
  (if Start
    (Audio|Components|Audio|Play _bobing)
    (else
      (Audio|Components|Audio|Stop _bobing)
      ;[0.15 0.15 0.15 0.5] Bobing Animation
      (bind _bobing_2 (Timeline|Bobing SetNewTime)
        (:Update
          (Transformation|SetRelativeLocation (Variables|Default|GetSphere) (Math|Vector|MakeVector 0.0 0.0 (* _bobing_2 (Variables|Default|GetBobDist))) false false))))))

(event Custom|CE_CheckInteract
  (bind _returnvalue (Transformation|GetActorLocation))
  ;[0.008726 0.05134 0.15 0.5] Interaction
  (if (not (Variables|Default|GetInteracting))
    (bind (_outhit _returnvalue_2) (Collision|SphereTraceByChannel _returnvalue _returnvalue 1e+02 "TraceTypeQuery1" false 0 "None"))
    (if _returnvalue_2
      (if (Utilities|DoesObjectImplementInterface (.HitActor (Collision|BreakHitResult _outhit)) "/Game/Components/BPI_Interactable.BPI_Interactable_C")
        (if (!= (Variables|Default|GetCurrentInteract) (.HitActor (Collision|BreakHitResult _outhit)))
          (Class|BPIInteractable|StopInteracting(Message) (Variables|Default|GetCurrentInteract))
          (bind _output_get (Variables|Default|SetCurrentInteract (.HitActor (Collision|BreakHitResult _outhit))))
          (Class|BPIInteractable|CanInteract(Message) _output_get))
        (elif (Utilities|IsValid (Variables|Default|GetCurrentInteract))
          (if (not (< (Transformation|GetDistanceTo (Variables|Default|GetCurrentInteract) self) 1e+02))
            (Class|BPIInteractable|StopInteracting(Message) (Variables|Default|GetCurrentInteract) :!label _label)
            (Variables|Default|SetCurrentInteract 0))))
      (elif (Utilities|IsValid (Variables|Default|GetCurrentInteract))
        (goto _label)))))

(event Input|EnhancedActionEvents|EnhancedInputActionIA_Move
  (params (ActionValue :type Vector%202D%20Structure) (ElapsedSeconds :type Float%20%28double-precision%29) (TriggeredSeconds :type Float%20%28double-precision%29) (InputAction :type Input%20Action%20Object%20Reference :default "/Game/Player/Input/IA_Move.IA_Move"))
  (bind (_x _y) (Math|Vector2D|BreakVector2D ActionValue))
  ;[0.15 0.15 0.15 0.5] Handle Move Input
  (if (not (Variables|Default|GetOnLand))
    (Pawn|Input|AddMovementInput (Math|Vector|MakeVector _x _y 0.0) 1.0 false)))

(event Input|EnhancedActionEvents|EnhancedInputActionIA_Jump
  (params (ActionValue :type Boolean) (ElapsedSeconds :type Float%20%28double-precision%29) (TriggeredSeconds :type Float%20%28double-precision%29) (InputAction :type Input%20Action%20Object%20Reference :default "/Game/Player/Input/IA_Jump.IA_Jump"))
  (bind _returnvalue (Transformation|GetActorLocation))
  ;[0.15 0.15 0.15 0.5] Handle Jump
  (if (and (or (Variables|Default|GetFloating) (Variables|Default|GetOnLand)) (not (Variables|Default|GetJumping)))
    (Variables|Default|SetJumping true)
    (CallFunction|AddVelocity 0.0 0.0 (Math|Float|Sqrt (* 1.5e+02 2.0 (* (Variables|Default|GetJumpHeight) 1e+03))))
    (Niagara|SpawnSystematLocation "/Game/VFX/NS_JumpSwirl.NS_JumpSwirl" (Math|Vector|MakeVector (.x _returnvalue) (.y _returnvalue) (+ (.z _returnvalue) (Variables|Default|GetJumpSpawn))) "0, 0, 0" "1.000000,1.000000,1.000000" true true "AutoRelease")
    (Utilities|FlowControl|Delay 0.5)
    (Variables|Default|SetJumping false)))

(event Input|EnhancedActionEvents|EnhancedInputActionIA_Interact
  (params (ActionValue :type Boolean) (ElapsedSeconds :type Float%20%28double-precision%29) (TriggeredSeconds :type Float%20%28double-precision%29) (InputAction :type Input%20Action%20Object%20Reference :default "/Game/Player/Input/IA_Interact.IA_Interact"))
  (bind _currentinteract (Variables|Default|GetCurrentInteract))
  ;[0.15 0.15 0.15 0.5] Handle Interact Input
  (if ActionValue
    (if (and (Variables|Default|GetInteracting) (Utilities|IsValid _currentinteract))
      (Class|BPIInteractable|Interact(Message) _currentinteract)
      (Variables|Default|SetInteracting true))
    (else
      (Utilities|FlowControl|Delay 0.5)
      (Variables|Default|SetInteracting false))))

(event EventTick
  (params (DeltaSeconds :type Float%20%28single-precision%29))
  (bind _returnvalue (Transformation|GetVelocity))
  ;[0.15 0.02177 0.02729 0.5] Update
  (Variables|Default|SetDeltaTime DeltaSeconds)
  (CallFunction|CEHandleGravity)
  (CallFunction|CECheckInteract)
  (CallFunction|CESetShadow)
  (Rendering|Material|SetVectorParameterValue "/Game/Materials/Global/MPC_Global.MPC_Global" "PlayerLocation" (Math|Conversions|ToLinearColor(Vector) (Transformation|GetWorldLocation (Variables|Default|GetCollision))) :!class /Script/Engine.KismetMaterialLibrary)
  (if (Variables|Default|GetJumping)
    (Variables|Default|SetCurrentVelocityMag 0.0)
    (else
      (Variables|Default|SetCurrentVelocityMag (/ (Math|Vector|VectorLength (Math|Vector|MakeVector (.x _returnvalue) (.y _returnvalue) 0.0)) (Class|MovementComponent|GetMaxSpeed (Variables|Default|GetFloatingPawnMovement)))))))

(event Custom|CE_SetMovement
  (bind _floatingpawnmovement (Variables|Default|GetFloatingPawnMovement))
  (Utilities|FlowControl|Sequence
    (:then_0
      (Variables|/Script/Engine.FloatingPawnMovement|SetMaxSpeed _floatingpawnmovement (Variables|Default|GetMaxSpeed)))
    (:then_1
      (Variables|/Script/Engine.FloatingPawnMovement|SetAcceleration _floatingpawnmovement (Variables|Default|GetAcceleration)))
    (:then_2
      (Variables|/Script/Engine.FloatingPawnMovement|SetDeceleration _floatingpawnmovement (Variables|Default|GetDeceleration)))))

(event EventBeginPlay
  (CallFunction|CEBobAnim)
  (CallFunction|CESetMovement)
  (Utilities|FlowControl|RetriggerableDelay 0.5)
  (CallFunction|CESetMovement)
  (bind _returnvalue (Actor|GetActorOfClass "/Game/Landscapes/WorldInteraction/BP_RippleManager.BP_RippleManager_C"))
  (Variables|Default|SetRippleManager _returnvalue)
  (bind _returnvalue_2 (Niagara|SpawnSystematLocation "/Game/VFX/NS_WaterSplash.NS_WaterSplash" "0, 0, 0" "0, 0, 0" "0.500000,0.500000,0.500000" false false "AutoRelease"))
  (bind _output_get (Variables|Default|SetSplash%20VFX _returnvalue_2))
  (Rendering|SceneCapture|ShowOnlyComponent (Variables|/Game/Landscapes/WorldInteraction/BP_RippleManager.BP_RippleManager_C|GetSceneCapture (Variables|Default|GetRippleManager)) _output_get))

(fn ConstructionScript)

(fn AddVelocity
  (params (X :type Float%20%28double-precision%29) (Y :type Float%20%28double-precision%29) (Z :type Float%20%28double-precision%29))
  (bind _floatingpawnmovement (Variables|Default|GetFloatingPawnMovement))
  (Variables|/Script/Engine.MovementComponent|SetVelocity _floatingpawnmovement (Math|Vector|MakeVector (+ (.x (Variables|/Script/Engine.MovementComponent|GetVelocity _floatingpawnmovement)) X) (+ (.y (Variables|/Script/Engine.MovementComponent|GetVelocity _floatingpawnmovement)) Y) (+ (.z (Variables|/Script/Engine.MovementComponent|GetVelocity _floatingpawnmovement)) Z))))

(fn CheckforWater
  (params (Hit :type Hit%20Result%20Structure))
  (return (Utilities|IsValid (Actor|GetComponentbyClass (.HitActor (Collision|BreakHitResult Hit)) "/Game/Components/Geo/AC_Flow.AC_Flow_C"))))