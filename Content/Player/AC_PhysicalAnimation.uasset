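; Actor component for the player character that blends physics simulation into the skeletal mesh's animation.
; On BeginPlay it creates a PhysicalAnimationComponent on the owner, links it to the mesh and binds to the player's jump dispatchers.
; Jumping sets full physics blend weight below "Bone", and stopping restores a light blend.
; A separate toggle event, uncalled here, only switches simulation on at that light blend.
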(event Custom|CE_TogglePhysicalAnimation
  (Class|SkeletalMeshComponent|SetAllBodiesBelowSimulatePhysics (Variables|Default|GetMesh) (Utilities|Name|MakeLiteralName "Bone") true false)
  (Class|SkeletalMeshComponent|SetAllBodiesBelowPhysicsBlendWeight (Variables|Default|GetMesh) (Utilities|Name|MakeLiteralName "Bone") 0.2 false true))

(event Custom|CE_SetBlendtoFull
  (Class|SkeletalMeshComponent|SetAllBodiesBelowPhysicsBlendWeight (Variables|Default|GetMesh) (Utilities|Name|MakeLiteralName "Bone") 1.0 false true))

(event Custom|CE_SetBlendtoNone
  (Class|SkeletalMeshComponent|SetAllBodiesBelowPhysicsBlendWeight (Variables|Default|GetMesh) (Utilities|Name|MakeLiteralName "Bone") 0.2 false true))

(event EventBeginPlay
  (bind _returnvalue (Components|GetOwner))
  (bind _asbp_player_character (Utilities|Casting|CastToBP_PlayerCharacter _returnvalue))
  (Variables|Default|SetPlayer _asbp_player_character)
  (bind _returnvalue_2 (Game|AddComponentbyClass _returnvalue "/Script/Engine.PhysicalAnimationComponent"))
  (bind _output_get (Variables|Default|SetPhysical%20Animation%20Component _returnvalue_2))
  (Class|PhysicalAnimationComponent|SetSkeletalMeshComponent _output_get (Variables|/Game/Player/BP_PlayerCharacter.BP_PlayerCharacter_C|GetMesh _asbp_player_character))
  (Variables|Default|SetMesh (Variables|/Game/Player/BP_PlayerCharacter.BP_PlayerCharacter_C|GetMesh _asbp_player_character))
  (EventDispatchers|BindEventtoEDJumping (Variables|Default|GetPlayer) (delegate Custom|CE_SetBlendtoFull))
  (EventDispatchers|BindEventtoEDStopJumping (Variables|Default|GetPlayer) (delegate Custom|CE_SetBlendtoNone)))

(event EventTick
  (params (DeltaSeconds :type Float%20%28single-precision%29)))