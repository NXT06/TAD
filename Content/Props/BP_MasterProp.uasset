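; Base prop actor that hovers above surfaces carrying an AC_Flow component and highlights when interactable.
; Each tick, a downward trace from the capsule disables gravity over such surfaces and adds upward force when too close, otherwise restoring gravity.
; The debug trace's hit color reflects the float state.
; Interaction events toggle the cube's custom depth and print debug text, while Interact itself is an empty stub.
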(event Custom|CE_HandleGravity
  (bind _returnvalue (Transformation|GetActorLocation))
  (bind _capsule (Variables|Default|GetCapsule))
  ;[0.1463 0.02158 0.15 0.5] Handle Gravity
  (Utilities|FlowControl|Sequence
    (:then_0
      (bind (_outhit _returnvalue_2) (Collision|LineTraceByChannel _returnvalue (- _returnvalue (Math|Vector|MakeVector 0.0 0.0 (+ (Components|Capsule|GetScaledCapsuleHalfHeight (Variables|Default|GetCapsule)) (Variables|Default|GetDistFromGround)))) "TraceTypeQuery1" false 0 "ForOneFrame" true (Variables|Default|GetTrace%20Hit%20Color) (Variables|Default|GetTrace%20Hit%20Color)))
      (if _returnvalue_2
        (bind _result (CallFunction|CheckforSurface _outhit))
        (if _result
          (if (< (.Distance (Collision|BreakHitResult _outhit)) (+ (Variables|Default|GetDistFromGround) (Variables|Default|GetLevelDist)))
            (Variables|Default|SetFloating true)
            (Physics|SetEnableGravity _capsule false)
            (Physics|AddForce (Variables|Default|GetCapsule) (Math|Vector|MakeVector 0.0 0.0 (* 1.0 (Variables|Default|GetFloatForce))) "None" false)
            (else
              (Variables|Default|SetFloating true)
              (Physics|SetEnableGravity _capsule false)))
          (else
            (Variables|Default|SetFloating false :!label _label)
            (Variables|Default|SetGravityMult (+ (Variables|Default|GetGravityMult) (Variables|Default|GetDelta%20Time)))
            (Physics|SetEnableGravity (Variables|Default|GetCapsule) true)))
        (else
          (goto _label))))
    (:then_1
      ;[0.15 0.15 0.15 0.5] Trace Color
      (if (Variables|Default|GetFloating)
        (if (< (.Distance (Collision|BreakHitResult _outhit)) (+ (Variables|Default|GetDistFromGround) (Variables|Default|GetLevelDist)))
          (Variables|Default|SetTrace%20Hit%20Color "(R=1.000000,G=0.985951,B=0.125357,A=1.000000)")
          (else
            (Variables|Default|SetTrace%20Hit%20Color "(R=0.025765,G=1.000000,B=0.184122,A=1.000000)")))
        (else
          (Variables|Default|SetTrace%20Hit%20Color "(R=1.000000,G=0.000000,B=0.056839,A=1.000000)"))))))

(event EventBeginPlay)

(event EventTick
  (params (DeltaSeconds :type Float%20%28single-precision%29))
  (Variables|Default|SetDelta%20Time DeltaSeconds)
  (CallFunction|CEHandleGravity))

(event EventInteract)

(event EventCanInteract
  (Development|PrintString "StartInteract")
  (Rendering|SetRenderCustomDepth (Variables|Default|GetCube) true))

(event EventStopInteracting
  (Development|PrintString "StopInteract")
  (Rendering|SetRenderCustomDepth (Variables|Default|GetCube) false))

(fn ConstructionScript)

(fn AddVelocity
  (params (X :type Float%20%28double-precision%29) (Y :type Float%20%28double-precision%29) (Z :type Float%20%28double-precision%29)))

(fn CheckforSurface
  (params (Hit :type Hit%20Result%20Structure))
  (return (Utilities|IsValid (Actor|GetComponentbyClass (.HitActor (Collision|BreakHitResult Hit)) "/Game/Components/Geo/AC_Flow.AC_Flow_C"))))