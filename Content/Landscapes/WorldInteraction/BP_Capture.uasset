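; Actor that keeps a player-following orthographic capture area and a persistent render target for landscape world interaction.
; At a set rate, it moves with the player in XY, snapped to a 1/256-of-width grid to keep texels stable.
; It then draws M_DrawToPersistent into RT_Persistent, passing the normalized move offset to compensate for the shift.
; Capture size and location are published to MPC_Capture for materials, and both render targets clear on BeginPlay.
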(event EventBeginPlay
  (bind _returnvalue (Actor|GetActorOfClass "/Game/Player/BP_PlayerCharacter.BP_PlayerCharacter_C"))
  (Variables|Default|SetPlayer _returnvalue)
  (Rendering|Material|SetScalarParameterValue "/Game/Landscapes/WorldInteraction/MPC_Capture.MPC_Capture" "CaptureSize" (Variables|/Script/Engine.SceneCaptureComponent2D|GetOrthoWidth (Variables|Default|GetSceneCapture)) :!class /Script/Engine.KismetMaterialLibrary)
  (bind _returnvalue_2 (Rendering|Material|CreateDynamicMaterialInstance "/Game/Landscapes/WorldInteraction/M_DrawToPersistent.M_DrawToPersistent" "None" "None" :!class /Script/Engine.KismetMaterialLibrary))
  (Variables|Default|SetDrawMaterial _returnvalue_2)
  (Rendering|ClearRenderTarget2D "/Game/Landscapes/WorldInteraction/RT_Capture.RT_Capture")
  (Rendering|ClearRenderTarget2D "/Game/Landscapes/WorldInteraction/RT_Persistent.RT_Persistent"))

(event EventTick
  (params (DeltaSeconds :type Float%20%28single-precision%29))
  (bind _output_get (Variables|Default|SetTimer (+ DeltaSeconds (Variables|Default|GetTimer))))
  (if (> _output_get (Variables|Default|GetCaptureRate))
    (CallFunction|MoveCapture)
    (CallFunction|DrawtoPersistant)
    (Variables|Default|SetTimer 0.0)))

(fn ConstructionScript)

(fn DrawtoPersistant
  (bind _scenecapture (Variables|Default|GetSceneCapture))
  (bind _move_offset (Variables|Default|GetMove%20Offset))
  (bind _orthowidth (Variables|/Script/Engine.SceneCaptureComponent2D|GetOrthoWidth _scenecapture))
  (bind _returnvalue (/ _move_offset _orthowidth))
  (Rendering|Material|SetVectorParameterValue (Variables|Default|GetDrawMaterial) "Offset" (Utilities|Struct|MakeLinearColor (.x _returnvalue) (.y _returnvalue) 0.0 1.0) :!class /Script/Engine.MaterialInstanceDynamic)
  (Rendering|DrawMaterialtoRenderTarget "/Game/Landscapes/WorldInteraction/RT_Persistent.RT_Persistent" (Variables|Default|GetDrawMaterial)))

(fn MoveCapture
  (bind _returnvalue (Transformation|GetActorLocation))
  (bind _returnvalue_2 (/ 1.0 256.0))
  (bind _scenecapture (Variables|Default|GetSceneCapture))
  (bind _player (Variables|Default|GetPlayer))
  (bind _returnvalue_3 (Transformation|GetActorLocation _player))
  (bind _orthowidth (Variables|/Script/Engine.SceneCaptureComponent2D|GetOrthoWidth _scenecapture))
  (bind _returnvalue_4 (* _orthowidth _returnvalue_2))
  (bind _returnvalue_5 (Class|KismetMathLibrary|VectorSnappedtoGrid (Math|Vector|MakeVector (.x _returnvalue_3) (.y _returnvalue_3) 0.0) _returnvalue_4))
  (bind _returnvalue_6 (- _returnvalue_5 _returnvalue))
  (bind _output_get (Variables|Default|SetMove%20Offset (Math|Vector2D|MakeVector2D (.x _returnvalue_6) (.y _returnvalue_6))))
  (Transformation|AddActorWorldOffset (Math|Vector|MakeVector (.x _output_get) (.y _output_get) 0.0))
  (Rendering|Material|SetVectorParameterValue "/Game/Landscapes/WorldInteraction/MPC_Capture.MPC_Capture" "CaptureLocation" (Math|Conversions|ToLinearColor(Vector) (Transformation|GetActorLocation)) :!class /Script/Engine.KismetMaterialLibrary))