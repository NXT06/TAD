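; Ripple manager that spawns ripple sprites at the player's location for a scene capture, with RT_Ripples cleared at start.
; BeginPlay pre-spawns a hidden sprite pool as show-only actors for the capture and publishes its width to MPC_Capture.
; Tick recycles sprites round-robin, more often as player velocity rises.
; MoveCaptureArea, not called here, follows the player in 1/256-width grid steps and publishes the capture location.
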(event EventBeginPlay
  (Rendering|Material|SetScalarParameterValue "/Game/Landscapes/WorldInteraction/MPC_Capture.MPC_Capture" "CaptureSize" (Variables|/Script/Engine.SceneCaptureComponent2D|GetOrthoWidth (Variables|Default|GetSceneCapture)) :!class /Script/Engine.KismetMaterialLibrary)
  (Rendering|ClearRenderTarget2D "/Game/Landscapes/WorldInteraction/RT_Ripples.RT_Ripples")
  (bind _returnvalue (Actor|GetActorOfClass "/Game/Player/BP_PlayerCharacter.BP_PlayerCharacter_C"))
  (Variables|Default|SetPlayer _returnvalue)
  (for _index (range 0 (- (Variables|Default|GetPoolSize) 1))
    (bind _returnvalue_2 (Game|SpawnActorfromClass "/Game/Landscapes/WorldInteraction/BP_RippleSprite.BP_RippleSprite_C" (Math|Transform|MakeTransform "0.000000,0.000000,100.000000" "0, 0, 0" "1.000000,1.000000,1.000000") "AlwaysSpawn" "MultiplyWithRoot" 0 0))
    (Rendering|SetActorHiddenInGame _returnvalue_2 true)
    (Rendering|SceneCapture|ShowOnlyActorComponents (Variables|Default|GetSceneCapture) _returnvalue_2 false)
    (Utilities|Array|Add (Variables|Default|GetRipplePool) _returnvalue_2)))

(event EventTick
  (params (DeltaSeconds :type Float%20%28single-precision%29))
  (bind _output_get (Variables|Default|SetTimer (+ DeltaSeconds (Variables|Default|GetTimer))))
  (if (> _output_get (- 1.05 (Variables|/Game/Player/BP_PlayerCharacter.BP_PlayerCharacter_C|GetCurrentVelocityMag (Variables|Default|GetPlayer))))
    (CallFunction|ActivateRipplefromPool)
    (Variables|Default|SetTimer 0.0)))

(fn ConstructionScript)

(fn ActivateRipplefromPool
  (Transformation|Teleport (Utilities|Array|Get(acopy) (Variables|Default|GetRipplePool) (Variables|Default|GetPoolIndex)) (Transformation|GetActorLocation (Variables|Default|GetPlayer)) "0, 0, 0")
  (Rendering|SetActorHiddenInGame (Utilities|Array|Get(acopy) (Variables|Default|GetRipplePool) (Variables|Default|GetPoolIndex)) false)
  (Default|CEResetRipple (Utilities|Array|Get(acopy) (Variables|Default|GetRipplePool) (Variables|Default|GetPoolIndex)))
  (bind _result (Math|Integer|IncrementInt (Variables|Default|GetPoolIndex))
    (:%20%20
      (Variables|Default|SetPoolIndex (Math|Integer|%(Integer) _result (Variables|Default|GetPoolSize))))))

(fn MoveCaptureArea
  (bind _returnvalue (Transformation|GetActorLocation))
  (bind _returnvalue_2 (/ 1.0 256.0))
  (bind _player (Variables|Default|GetPlayer))
  (bind _scenecapture (Variables|Default|GetSceneCapture))
  (bind _returnvalue_3 (Transformation|GetActorLocation _player))
  (bind _orthowidth (Variables|/Script/Engine.SceneCaptureComponent2D|GetOrthoWidth _scenecapture))
  (bind _returnvalue_4 (* _orthowidth _returnvalue_2))
  (bind _returnvalue_5 (Class|KismetMathLibrary|VectorSnappedtoGrid (Math|Vector|MakeVector (.x _returnvalue_3) (.y _returnvalue_3) 0.0) _returnvalue_4))
  (bind _returnvalue_6 (- _returnvalue_5 _returnvalue))
  (bind _output_get (Variables|Default|SetMoveOffset (Math|Vector2D|MakeVector2D (.x _returnvalue_6) (.y _returnvalue_6))))
  (Transformation|AddActorWorldOffset (Math|Vector|MakeVector (.x _output_get) (.y _output_get) 0.0))
  (Rendering|Material|SetVectorParameterValue "/Game/Landscapes/WorldInteraction/MPC_Capture.MPC_Capture" "CaptureLocation" (Math|Conversions|ToLinearColor(Vector) (Transformation|GetActorLocation)) :!class /Script/Engine.KismetMaterialLibrary))