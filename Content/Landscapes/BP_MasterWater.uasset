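; Base-style water actor that can push overlapping objects when its ACWater component is set to flowing.
; Cube overlap begin and end send move and stop messages, passing ACWater, to the other actor's first BPI_Moveable component.
; Debug cones show the actor's forward vector during construction and the negated flow direction at BeginPlay.
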(event OnComponentBeginOverlap(Cube)
  (params (OverlappedComponent :type Primitive%20Component%20Object%20Reference) (OtherActor :type Actor%20Object%20Reference) (OtherComp :type Primitive%20Component%20Object%20Reference) (OtherBodyIndex :type Integer) (bFromSweep :type Boolean) (SweepResult :type Hit%20Result%20Structure%20%28by%20ref%29))
  (Utilities|FlowControl|Sequence
    (:then_0
      (if (Variables|/Game/Components/Geo/AC_Flow.AC_Flow_C|GetFlowing (Variables|Default|GetAC_Water))
        (Class|BPIMoveable|Move(Message) (Utilities|Array|Get(acopy) (Class|Actor|GetComponentsbyInterface OtherActor "/Game/Components/BPI_Moveable.BPI_Moveable_C")) (Variables|Default|GetAC_Water))))))

(event OnComponentEndOverlap(Cube)
  (params (OverlappedComponent :type Primitive%20Component%20Object%20Reference) (OtherActor :type Actor%20Object%20Reference) (OtherComp :type Primitive%20Component%20Object%20Reference) (OtherBodyIndex :type Integer))
  (Utilities|FlowControl|Sequence
    (:then_0
      (if (Variables|/Game/Components/Geo/AC_Flow.AC_Flow_C|GetFlowing (Variables|Default|GetAC_Water))
        (Class|BPIMoveable|StopMove(Message) (Utilities|Array|Get(acopy) (Class|Actor|GetComponentsbyInterface OtherActor "/Game/Components/BPI_Moveable.BPI_Moveable_C")) (Variables|Default|GetAC_Water))))))

(event EventBeginPlay
  (bind _returnvalue (Transformation|GetActorLocation))
  (bind _ac_water (Variables|Default|GetAC_Water))
  (bind _direction (Variables|/Game/Components/Geo/AC_Flow.AC_Flow_C|GetDirection _ac_water))
  (bind _returnvalue_2 (Math|Vector|NegateVector _direction))
  (Class|KismetSystemLibrary|DrawDebugConeinDegrees _returnvalue _returnvalue_2 1e+02 1e+01 1e+01 1 "(R=1.000000,G=1.000000,B=1.000000,A=1.000000)" 1e+03 2.0)
  (Class|KismetSystemLibrary|DrawDebugConeinDegrees (+ _returnvalue (* _returnvalue_2 1e+02)) _returnvalue_2 1e+02 1e+01 1e+01 1 "(R=1.000000,G=1.000000,B=1.000000,A=1.000000)" 1e+03 2.0))

(event Collision|EventActorBeginOverlap
  (params (OtherActor :type Actor%20Object%20Reference)))

(fn ConstructionScript
  (Class|KismetSystemLibrary|DrawDebugConeinDegrees (Transformation|GetActorLocation) (Math|Vector|GetForwardVector (Transformation|GetActorRotation)) 4e+02 2e+01 2e+01 4 "(R=1.000000,G=1.000000,B=1.000000,A=1.000000)" 0.1 3.0))