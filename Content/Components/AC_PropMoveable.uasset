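; AC_PropMoveable is an actor component that lets water flow push its owning prop.
; Move takes direction and speed from the water movement data and enables tick, which applies a scaled force to the owner's capsule.
; StopMove scans overlapping BP_MasterWater actors for a flowing AC_Flow, but as wired clears movement and disables tick either way.
; Both events act after a short delay.
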(event EventStopMove
  (params (AC%20Flow :type AC%20Flow%20Object%20Reference))
  (bind _collider (Variables|Default|GetCollider))
  (bind _overlappingactors (Collision|GetOverlappingActors _collider "/Game/Landscapes/BP_MasterWater.BP_MasterWater_C" :!class /Script/Engine.PrimitiveComponent))
  (Utilities|FlowControl|Delay 0.2)
  (if (> (Utilities|Array|Length _overlappingactors) 0)
    (bind _array_element (Utilities|Array|ForEachLoopwithBreak _overlappingactors :!label _label)
      (:LoopBody
        (if (Variables|/Game/Components/Movement/AC_Flow.AC_Flow_C|GetFlowing (Actor|GetComponentbyClass _array_element "/Game/Components/Movement/AC_Flow.AC_Flow_C"))
          (goto _label Break)))
      (:Completed
        (Variables|Default|SetActive false :!label _label_2)
        (Variables|Default|SetSpeed 0.0)
        (Variables|Default|SetDirection "0, 0, 0")
        (Components|Tick|SetComponentTickEnabled false)))
    (else
      (goto _label_2))))

(event EventMove
  (params (WaterMovement :type AC%20Flow%20Object%20Reference) (Impulse :type Boolean) (ImpulseMovement :type AC%20Impulse%20Object%20Reference))
  (Utilities|FlowControl|Delay 0.2)
  (Development|PrintString "Start Move")
  (Components|Tick|SetComponentTickEnabled true)
  (Variables|Default|SetActive true)
  (Variables|Default|SetDirection (Variables|/Game/Components/Movement/AC_Flow.AC_Flow_C|GetDirection WaterMovement))
  (Variables|Default|SetSpeed (Variables|/Game/Components/Movement/AC_Flow.AC_Flow_C|GetSpeed WaterMovement)))

(event EventBeginPlay
  (Variables|Default|SetOwner (Actor|GetComponentbyClass (Components|GetOwner) "/Script/Engine.CapsuleComponent"))
  (Variables|Default|SetCollider (Actor|GetComponentbyClass (Components|GetOwner) "/Script/Engine.CapsuleComponent")))

(event EventTick
  (params (DeltaSeconds :type Float%20%28single-precision%29))
  (if (Variables|Default|GetActive)
    (Physics|AddForce (Variables|Default|GetOwner) (* (* (Variables|Default|GetDirection) (Variables|Default|GetSpeed)) 5e+02) "None" false)))