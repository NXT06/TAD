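; Actor component that spawns water-style ripple sprites beneath its owner as it moves, using an object pool.
; BeginPlay pre-spawns hidden BP_RippleSprite actors and registers each with the BP_RippleManager scene capture's show-only list.
; Tick accumulates time and fires faster as horizontal speed nears MaxSpeed.
; Each firing teleports the next pooled sprite to the owner, unhides and resets it, cycling the pool index round-robin.
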(event EventBeginPlay
  (bind _ripple_start_size (Variables|Default|GetRipple%20Start%20Size))
  (for _index (range 0 (- (Variables|Default|GetPool%20size) 1))
    (bind _returnvalue (Game|SpawnActorfromClass "/Game/Landscapes/WorldInteraction/BP_RippleSprite.BP_RippleSprite_C" (Math|Transform|MakeTransform "0.000000,0.000000,100.000000" "0, 0, 0" (Math|Vector|MakeVector _ripple_start_size 1.0 _ripple_start_size)) "AlwaysSpawn" "MultiplyWithRoot" 0 0))
    (Rendering|SetActorHiddenInGame _returnvalue true)
    (bind _returnvalue_2 (Actor|GetActorOfClass "/Game/Landscapes/WorldInteraction/BP_RippleManager.BP_RippleManager_C"))
    (Rendering|SceneCapture|ShowOnlyActorComponents (Variables|/Game/Landscapes/WorldInteraction/BP_RippleManager.BP_RippleManager_C|GetSceneCapture _returnvalue_2) _returnvalue false)
    (Utilities|Array|Add (Variables|Default|GetRipple%20Pool) _returnvalue)))

(event EventTick
  (params (DeltaSeconds :type Float%20%28single-precision%29))
  (bind _returnvalue (Components|GetOwner))
  (bind _returnvalue_2 (Transformation|GetVelocity _returnvalue))
  (bind _output_get (Variables|Default|SetTimer (+ DeltaSeconds (Variables|Default|GetTimer))))
  (if (> _output_get (- 1.05 (/ (Math|Vector|VectorLength (Math|Vector|MakeVector (.x _returnvalue_2) (.y _returnvalue_2) 0.0)) (Variables|Default|GetMaxSpeed))))
    (CallFunction|ActivateRipplefromPool)
    (Variables|Default|SetTimer 0.0)))

(fn ActivateRipplefromPool
  (Transformation|Teleport (Utilities|Array|Get(acopy) (Variables|Default|GetRipple%20Pool) (Variables|Default|GetPool%20Index)) (Transformation|GetActorLocation (Components|GetOwner)) "0, 0, 0")
  (Rendering|SetActorHiddenInGame (Utilities|Array|Get(acopy) (Variables|Default|GetRipple%20Pool) (Variables|Default|GetPool%20Index)) false)
  (Default|CEResetRipple (Utilities|Array|Get(acopy) (Variables|Default|GetRipple%20Pool) (Variables|Default|GetPool%20Index)))
  (bind _result (Math|Integer|IncrementInt (Variables|Default|GetPool%20Index))
    (:%20%20
      (Variables|Default|SetPool%20Index (Math|Integer|%(Integer) _result (Variables|Default|GetPool%20size))))))