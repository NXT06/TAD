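; Actor component that lets flow forces push its owning pawn through the owner's FloatingPawnMovement.
; Move and StopMove add or remove flows, each change recomputing a normalized summed direction and taking the strongest speed.
; Speeds above one also scale up the pawn's base max speed.
; Tick applies forced input along that direction with a debug arrow, switching on when flows are added and off when none remain.
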(event EventMove
  (params (Movement :type AC%20Flow%20Object%20Reference))
  (bind _currentforces (Variables|Default|GetCurrentForces))
  (if (Utilities|Array|ContainsItem _currentforces Movement)
    (Development|PrintString "Already Moving Player")
    (else
      (Utilities|Array|Add _currentforces Movement)
      (CallFunction|CalculateMovement (Variables|Default|GetCurrentForces))
      (Utilities|FlowControl|DelayUntilNextTick)
      (Development|PrintString "Added New Flow")
      (Components|Tick|SetComponentTickEnabled true))))

(event EventBeginPlay
  (bind _output_get (Variables|Default|SetFloating%20Pawn (Actor|GetComponentbyClass (Components|GetOwner) "/Script/Engine.FloatingPawnMovement")))
  (Variables|Default|SetMax%20Speed (Variables|/Script/Engine.FloatingPawnMovement|GetMaxSpeed _output_get))
  (Variables|Default|SetCollider (Actor|GetComponentbyClass (Components|GetOwner) "/Script/Engine.CapsuleComponent")))

(event EventTick
  (params (DeltaSeconds :type Float%20%28single-precision%29))
  (bind _collider (Variables|Default|GetCollider))
  (bind _returnvalue (Transformation|GetWorldLocation _collider))
  (Class|PawnMovementComponent|AddInputVector (Variables|Default|GetFloating%20Pawn) (* (Variables|Default|GetCurrent%20Speed) (Variables|Default|GetCumulativeDirection)) true)
  (Rendering|Debug|DrawDebugArrow _returnvalue (+ _returnvalue (* (+ (Variables|Default|GetCurrent%20Speed) 1e+02) (Variables|Default|GetCumulativeDirection))) 5e+01 "(R=0.058500,G=1.000000,B=0.052993,A=1.000000)" 0.01 5.0))

(event EventStopMove
  (params (AC%20Flow :type AC%20Flow%20Object%20Reference))
  (bind _currentforces (Variables|Default|GetCurrentForces))
  (if (Utilities|Array|ContainsItem _currentforces AC%20Flow)
    (bind _returnvalue (Utilities|Array|RemoveItem _currentforces AC%20Flow))
    (if _returnvalue
      (CallFunction|CalculateMovement (Variables|Default|GetCurrentForces))
      (Development|PrintString "Removed Flow")
      (if (< (Utilities|Array|Length (Variables|Default|GetCurrentForces)) 1)
        (Components|Tick|SetComponentTickEnabled false))
      (else
        (Development|PrintString "Failed to Remove Flow")))
    (else
      (Development|PrintString "Failed to find Flow"))))

(fn CalculateMovement
  (params (Flows :type Array%20of%20AC%20Flow%20Object%20References))
  (bind _floating_pawn (Variables|Default|GetFloating%20Pawn))
  (Variables|/Script/Engine.FloatingPawnMovement|SetMaxSpeed (Variables|Default|GetFloating%20Pawn) (Variables|Default|GetMax%20Speed))
  (Variables|Default|SetCumulativeDirection "0, 0, 0")
  (Variables|Default|SetCurrent%20Speed 0.0)
  (for _array_element Flows
    (Variables|Default|SetCumulativeDirection (+ (Variables|Default|GetCumulativeDirection) (Variables|/Game/Components/Geo/AC_Flow.AC_Flow_C|GetDirection _array_element)))
    (if (> (Variables|/Game/Components/Geo/AC_Flow.AC_Flow_C|GetSpeed _array_element) (Variables|Default|GetCurrent%20Speed))
      (Variables|Default|SetCurrent%20Speed (Variables|/Game/Components/Geo/AC_Flow.AC_Flow_C|GetSpeed _array_element))))
  (Variables|Default|SetCumulativeDirection (Math|Vector|Normalize (Variables|Default|GetCumulativeDirection)))
  (Development|PrintString (Utilities|String|ToString(Integer) (Utilities|Array|Length (Variables|Default|GetCurrentForces))))
  (if (> (Variables|Default|GetCurrent%20Speed) 1.0)
    (Variables|/Script/Engine.FloatingPawnMovement|SetMaxSpeed _floating_pawn (* (Variables|Default|GetCurrent%20Speed) (Class|MovementComponent|GetMaxSpeed _floating_pawn)))))